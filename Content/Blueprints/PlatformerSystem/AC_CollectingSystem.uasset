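; AC_CollectingSystem is a coin counter, apparently an actor component, in the platformer system.
; AddCoin adds an amount to Coins and caps the total at MaxCoins.
; Remove takes no amount and adds zero before clamping at zero, so it does not actually subtract coins.
; Tick prints the current and maximum coin counts on screen every frame through PrintString.
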(event `self.ReceiveTick`
  (params (DeltaSeconds :type "Float (single-precision)"))
  (`KismetSystemLibrary.PrintString` (`KismetStringLibrary.Concat_StrStr` "COINS:" (`KismetStringLibrary.Conv_IntToString` (`self.Coins`)) "/" (`KismetStringLibrary.Conv_IntToString` (`self.MaxCoins`))) true true (struct :`G` 0.66 :`B` 1.0 :`A` 1.0) 0.0))

(event `AddCoin`
  (params (Amount :type Integer))
  (bind _output_get (set `self.Coins` (+ (stale _output_get) Amount)))
  (if (> (`self.Coins`) (`self.MaxCoins`))
    (set `self.Coins` (`self.MaxCoins`))))

(event `Remove`
  (bind _output_get (set `self.Coins` (+ (stale _output_get) 0)))
  (if (< (`self.Coins`) 0)
    (set `self.Coins` 0)))